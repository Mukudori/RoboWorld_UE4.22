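; CommandController is a Python-backed component that turns text commands into action ID arrays for the UserController.
; ExecuteFromString runs the Model component's LSTM, gets actions from Python, converts them to integers and flags a new command.
; ExecuteFromIndex stores that array on the UserController and returns Python's rebuilt command string; helpers wrap action and word lookups and Vocabulary CSV data.
; The empty-list error never fires because the length check is >= 0.
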(event `self.ReceiveBeginPlay`
  (bind _asuser_controller (cast `/Game/Blueprint/UserController` (`GameplayStatics.GetPlayerController` 0)))
  (set `self.UserController` _asuser_controller))

(fn `CheckAction`
  (params (ActionID :type Integer))
  (returns (isAction :type Boolean))
  (bind _returnvalue (`self.CallPythonComponentMethodBool` "isAction" (`KismetStringLibrary.Conv_IntToString` ActionID)))
  (return _returnvalue))

(fn `ExecuteFromIndex`
  (params (CommandIndex :type "Array of Integer"))
  (returns (OutputMessage :type String))
  (locals (defaultString :type String :default "Функция команды не создана") (Subject :type Integer) (Context :type Integer) (LastPosition :type Integer))
  (set `/Game/Blueprint/UserController.CommandArray` CommandIndex (`self.UserController`))
  (bind _returnvalue (`self.CallPythonComponentMethodString` "getCommandStringFromIdsArray" (`self.CommandString`)))
  (return _returnvalue))

(fn `ExecuteFromString`
  (params (Command :type String))
  (returns (outputMessage :type String))
  (locals (DebugString :type String :default "Индекс действия : "))
  ;[1 1 1] Запуск модели
  (`/Game/Blueprint/Python/Model.runLSTMModel` (`Actor.GetComponentByClass` (`GameplayStatics.GetPlayerController` 0) "/Game/Blueprint/Python/Model.Model_C") Command)
  (bind _output_strings (`self.CallPythonComponentMethodStringArray` "getActionListFromCommandString" Command))
  (bind _actionintarray (`self.StringArrayToIntArray` _output_strings))
  (if (>= (`KismetArrayLibrary.Array_Length` _actionintarray) 0)
    (bind _outputmessage (`self.ExecuteFromIndex` _actionintarray))
    (`/Game/Blueprint/UserController.SetNewCommand` (`self.UserController`) true)
    (return _outputmessage)
    (else
      (`KismetSystemLibrary.PrintString` "Python вернул пустой список действий " true true (struct :`R` 1.0 :`B` 0.064177 :`A` 1.0)))))

(fn `GetWordFromID`
  (params (ID_Word :type Integer))
  (returns (Word :type String))
  (bind _returnvalue (`self.CallPythonComponentMethodString` "getWordFromID" (`KismetStringLibrary.Conv_IntToString` ID_Word)))
  (return _returnvalue))

(fn `PrintPreprocessingTrainData`
  (returns (message :type String))
  (bind _alldata (`/Game/Blueprint/Python/Vocabulary.get_String_ALL_Data_From_CSV` (`Actor.GetComponentByClass` (`GameplayStatics.GetPlayerController` 0) "/Game/Blueprint/Python/Vocabulary.Vocabulary_C")))
  (return _alldata))

(fn `StringArrayToIntArray`
  (params (ActionStringArray :type "Array of String"))
  (returns (ActionIntArray :type "Array of Integer"))
  (locals (ActionArray :type "Array of Integer"))
  (bind _actionarray (`local.ActionArray`))
  (set `self.CommandString` "")
  (for (_array_element _array_index) ActionStringArray
    (bind _returnvalue (`self.CallPythonComponentMethodInt` "stringIntToInt" _array_element))
    (`KismetArrayLibrary.Array_Insert` _actionarray _returnvalue _array_index)
    (set `self.CommandString` (`KismetStringLibrary.Concat_StrStr` (`self.CommandString`) " " _array_element)))
  (return _actionarray))