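; Robot pawn, driven by a RobotAIController, that walks and handles cups and medicine.
; Tick runs the long action chosen by ID unless the controller stops it (walking with trace-based turning), and updates a physics-handle target.
; Pickups snap items to left or right hand sockets, though only LeftAttachedActor records them.
; Putting down finds items by tag, destroys them and spawns replacements ahead; GetWater and DropObject are empty, and perception prints sightings.
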(event `self.ReceiveBeginPlay`
  (bind _asrobot_aicontroller (cast `/Game/Blueprint/Robot/AI/RobotAIController` (`AIBlueprintHelperLibrary.GetAIController` self)))
  (set `self.AIController` _asrobot_aicontroller))

(event `self.ReceiveTick`
  (params (DeltaSeconds :type "Float (single-precision)"))
  (`|ExecutionSequence`
    (:`then_0`
      (`self.ExecuteLongActions`))
    (:`then_1`
      ;[1 1 1] Захват локации объекта
      (`PhysicsHandleComponent.SetTargetLocation` (`self.PhysicsHandle`) (`SceneComponent.K2_GetComponentLocation` (`self.Grab_Location`))))))

(event `Move`
  (params (Direction :type "Vector Structure") (Scale :type "Float (double-precision)"))
  ;[1 1 1] Передаижение по вектору
  (`self.AddMovementInput` Direction Scale))

(event `PickUpObject`
  (params (actor :type "Actor Object Reference") (socket :type Name))
  (bind _robotvision (`self.RobotVision`))
  (bind _returnvalue (`SceneComponent.K2_GetComponentLocation` _robotvision))
  ;[1 1 1] Поднять объект
  (`self.K2_AttachToActor` actor socket "KeepRelative" "KeepRelative" "KeepRelative")
  (bind (_outhit _returnvalue_2) (`KismetSystemLibrary.LineTraceSingleForObjects` :`Start` _returnvalue :`End` (+ _returnvalue (* (`SceneComponent.GetForwardVector` _robotvision) 250.0)) :`ObjectTypes` (`|MakeArray` "ObjectTypeQuery4" :!type "EObjectTypeQuery Enum") :`bTraceComplex` true :`DrawDebugType` "Persistent"))
  (if _returnvalue_2
    (`PhysicsHandleComponent.GrabComponentAtLocation` (`self.PhysicsHandle`) null "None" (0.0 0.0 0.0))))

(event `DropObject`)

(event `self.AIPerception.OnTargetPerceptionUpdated`
  (params (Actor :type "Actor Object Reference") (Stimulus :type "AIStimulus Structure")))

(event `self.PawnSensing.OnComponentActivated`
  (params (Component :type "ActorComponent Object Reference") (bReset :type Boolean)))

(event `self.AIPerception.OnPerceptionUpdated`
  (params (UpdatedActors :type "Array of Actor Object Reference (by ref)"))
  (for _array_element UpdatedActors
    (`KismetSystemLibrary.PrintString` (`KismetStringLibrary.Concat_StrStr` "Вижу " (`KismetSystemLibrary.GetDisplayName` _array_element) " "))))

(fn `CheckArm`
  (params (tag :type Name))
  (returns (id_arm :type Integer))
  (locals (check :type Boolean) (id :type Integer :default 0))
  (for _array_element (`Actor.Tags` (`self.LeftAttachedActor`))
    (if (== _array_element tag)
      (set `local.id` 1)
      ;[1 1 1] 1 = left, 2 = right, 0 = none
      (return (`local.id`))))
  (if (not (== (`local.id`) 1))
    (for _array_element_2 (`Actor.Tags` (`self.RightAttachedActor`))
      (if (== _array_element_2 tag)
        (set `local.id` 2))))
  (return (`local.id`)))

(fn `DetachArm`
  (params (arm_id :type Integer))
  (bind _rightattachedactor (`self.RightAttachedActor`))
  (bind _leftattachedactor (`self.LeftAttachedActor`))
  (switch `int` arm_id
    (:`1`
      (`SceneComponent.K2_DetachFromComponent` (`Actor.RootComponent` _leftattachedactor) "KeepRelative" "KeepRelative" "KeepRelative" true)
      (`self.K2_DestroyActor` _leftattachedactor)
      (set `self.LeftArmUsed` false))
    (:`2`
      (`SceneComponent.K2_DetachFromComponent` (`Actor.RootComponent` _rightattachedactor) "KeepRelative" "KeepRelative" "KeepRelative" true)
      (`self.K2_DestroyActor` _rightattachedactor)
      (set `self.RightArmUsed` false))))

(fn `ExecuteLongActions`
  (if (not (`/Game/Blueprint/Robot/AI/RobotAIController.StopAll` (`self.AIController`)))
    (switch `int` (`self.LongActionID`)
      (:`1`
        (`self.GoFront`)))))

(fn `ExecutePickUpObject`
  (params (actor :type "Actor Object Reference") (socket :type Name))
  (`SceneComponent.K2_AttachToComponent` (`Actor.RootComponent` actor) (`self.Mesh`) socket "SnapToTarget" "SnapToTarget" "SnapToTarget" true)
  (set `self.LeftAttachedActor` actor))

(fn `GetCup`
  (params (ActorOfCoup :type "Actor Object Reference"))
  (if (not (`self.LeftArmUsed`))
    (`self.ExecutePickUpObject` ActorOfCoup "left_cup")
    (set `self.LeftArmUsed` true)
    (`KismetSystemLibrary.PrintString` "Взял лекарство в левую руку")
    (elif (not (`self.RightArmUsed`))
      (`self.ExecutePickUpObject` ActorOfCoup "right_cup")
      (set `self.RightArmUsed` true)
      (`KismetSystemLibrary.PrintString` "Взял лекарство в правую руку")
      (else
        (`KismetSystemLibrary.PrintString` "Обе руки заняты")))))

(fn `GetTabletki`
  (params (tabletki :type "Actor Object Reference"))
  (if (not (`self.LeftArmUsed`))
    (`self.ExecutePickUpObject` tabletki "left_tabletki")
    (set `self.LeftArmUsed` true)
    (`KismetSystemLibrary.PrintString` "Взял лекарство в левую руку")
    (elif (not (`self.RightArmUsed`))
      (`self.ExecutePickUpObject` tabletki "right_tabletki")
      (set `self.RightArmUsed` true)
      (`KismetSystemLibrary.PrintString` "Взял лекарство в правую руку")
      (else
        (`KismetSystemLibrary.PrintString` "Обе руки заняты")))))

(fn `GetWater`)

(fn `GoFront`
  (locals (bufDir :type "Vector Structure"))
  (bind _returnvalue (`self.K2_GetActorLocation`))
  (`|ExecutionSequence`
    (:`then_0`
      (bind (_outhit _returnvalue_2) (`KismetSystemLibrary.LineTraceSingle` :`Start` _returnvalue :`End` (+ _returnvalue (* (`self.GetActorRightVector`) 500)) :`TraceChannel` "TraceTypeQuery1" :`DrawDebugType` "ForOneFrame"))
      (if _returnvalue_2
        (set `self.Direction` (`KismetMathLibrary.GreaterGreater_VectorRotator` (`self.Direction`) (struct :`Yaw` 1.0)))))
    (:`then_1`
      (`self.Move` (`self.Direction`) 0.5))))

(fn `PutCupWater`
  (locals (Cup_Tags :type "Array of Name"))
  (bind _id_arm (`self.CheckArm` "стакан"))
  (if (== _id_arm 0)
    (`KismetSystemLibrary.PrintString` "в руках нет этого предмета")
    (else
      (`self.DetachArm` _id_arm)
      (bind _returnvalue (`|SpawnActorFromClass` "/Game/Blueprint/using_actors/BP_Cup.BP_Cup_C" (`KismetMathLibrary.MakeTransform` (+ (`self.K2_GetActorLocation`) (* (`self.GetActorForwardVector`) 100))) "Undefined" "OverrideRootScale" null null))
      (set `Actor.Tags` (`local.Cup_Tags`) _returnvalue))))

(fn `PutTabletki`
  (locals (tabletki_tags :type "Array of Name") (check :type Boolean))
  (bind _id_arm (`self.CheckArm` "лекарство"))
  (if (== _id_arm 0)
    (`KismetSystemLibrary.PrintString` "в руках нет этого предмета")
    (else
      (`self.DetachArm` _id_arm)
      (bind _returnvalue (`|SpawnActorFromClass` "/Game/Blueprint/using_actors/BP_tabletki.BP_tabletki_C" (`KismetMathLibrary.MakeTransform` (+ (`self.K2_GetActorLocation`) (* (`self.GetActorForwardVector`) 100))) "Undefined" "OverrideRootScale" null null))
      (set `Actor.Tags` (`local.tabletki_tags`) _returnvalue))))

(fn `SetLongActonID`
  (params (LongActionID :type Integer))
  (set `self.LongActionID` LongActionID))

(fn `SetStopAll`
  (params (StopAll :type Boolean))
  (set `self.StopAll` StopAll))

(fn `UserConstructionScript`)