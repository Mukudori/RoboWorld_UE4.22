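; User is a player-controlled Blueprint that moves and rotates a camera from axis inputs.
; Look axes feed controller yaw and pitch, while movement axes add input along the actor's forward and right vectors, with forward input scaled up tenfold.
; Vertical movement uses the up vector of a yaw-only control rotation, keeping it world-vertical regardless of pitch.
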(event `InputAxis|Go TopDown`
  (params (AxisValue :type "Float (single-precision)"))
  ;[1 1 1] Управление камерой
  (`self.AddMovementInput` (`self.GetActorForwardVector`) (* AxisValue 10.0)))

(event `InputAxis|Look UP / Down`
  (params (AxisValue :type "Float (single-precision)"))
  ;[1 1 1] Управление камерой
  (`self.AddControllerPitchInput` AxisValue))

(event `InputAxis|Go Up / Down`
  (params (AxisValue :type "Float (single-precision)"))
  (bind (_returnvalue_roll _returnvalue_pitch _returnvalue_yaw) (`KismetMathLibrary.BreakRotator` (`self.GetControlRotation`)))
  ;[1 1 1] Управление камерой
  (`self.AddMovementInput` (`KismetMathLibrary.GetUpVector` (`KismetMathLibrary.MakeRotator` 0.0 0.0 _returnvalue_yaw)) AxisValue))

(event `InputAxis|Go RightLeft`
  (params (AxisValue :type "Float (single-precision)"))
  ;[1 1 1] Управление камерой
  (`self.AddMovementInput` (`self.GetActorRightVector`) AxisValue))

(event `InputAxis|Look Right / Left`
  (params (AxisValue :type "Float (single-precision)"))
  ;[1 1 1] Управление камерой
  (`self.AddControllerYawInput` AxisValue))

(fn `UserConstructionScript`)