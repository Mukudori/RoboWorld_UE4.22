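; UserController is the player controller that builds the robot-operation UI: a command terminal plus camera, memory and action-queue widgets.
; BeginPlay adds all four to the viewport and sets game-and-UI input focused on the terminal's text field.
; An input action toggles terminal visibility through a FlipFlop.
; Accessor functions expose a command array and a new-command value, and PrintMessageInTerminal forwards messages to the terminal.
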(event `self.ReceiveBeginPlay`
  (bind _userterminal (`self.UserTerminal`))
  ;[1 1 1] Создать и скрыть виджет терминала
  (bind _returnvalue (`|CreateWidget` "/Game/Blueprint/UI/UserTerminal.UserTerminal_C"))
  (bind _output_get (set `self.UserTerminal` _returnvalue))
  (`UserWidget.AddToViewport` _output_get 0)
  (`Widget.SetVisibility` _userterminal "Visible")
  (`WidgetBlueprintLibrary.SetInputMode_GameAndUIEx` self (`/Game/Blueprint/UI/UserTerminal.EditableText_491` _userterminal))
  ;[1 1 1] Виджет камеры робота
  (bind _returnvalue_2 (`|CreateWidget` "/Game/Blueprint/UI/RobotCamera.RobotCamera_C"))
  (`UserWidget.AddToViewport` _returnvalue_2 0)
  ;[1 1 1] Виджет памяти робота
  (bind _returnvalue_3 (`|CreateWidget` "/Game/Blueprint/UI/RobotMemory.RobotMemory_C"))
  (`UserWidget.AddToViewport` _returnvalue_3 0)
  ;[1 1 1] Виджет очереди действий
  (bind _returnvalue_4 (`|CreateWidget` "/Game/Blueprint/UI/ActionsList.ActionsList_C"))
  (bind _output_get_2 (set `self.ActionsListWidget` _returnvalue_4))
  (`UserWidget.AddToViewport` _output_get_2 0))

(event `InputAction|Show/Close User Terminal`
  (params (Key :type "Key Structure"))
  (bind _userterminal (`self.UserTerminal`))
  ;[1 1 1] Открыть/закрыть терминал
  (:`Pressed`
    (`/Engine/EditorBlueprintResources/StandardMacros.FlipFlop`
      (:`A`
        (`Widget.SetVisibility` _userterminal "Visible"))
      (:`B`
        (`Widget.SetVisibility` _userterminal "Hidden")))))

(fn `CheckNewCommand`
  (returns (newCommand :type Boolean))
  (return (`self.NewCommand`)))

(fn `GetCommandVector`
  (returns (ComArray :type "Array of Integer"))
  (return (`self.CommandArray`)))

(fn `PrintMessageInTerminal`
  (params (Message :type String))
  (`/Game/Blueprint/UI/UserTerminal.print_to_View` (`self.UserTerminal`) Message))

(fn `SetCommandVector`
  (params (InputCommands :type "Array of Integer"))
  (set `self.CommandArray` InputCommands))

(fn `SetNewCommand`
  (params (newCommand :type Boolean))
  (set `self.NewCommand` newCommand))

(fn `UserConstructionScript`)